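; BP_Rebound is a bumper-style actor that knocks away whatever hits it and awards points for the hit.
; BeginPlay caches the first player controller as PC_IronSpin.
; On Hit, it applies an impulse to the other component at the impact location along the negated hit normal, scaled by ReboundStrenght.
; The same strength, truncated to an integer, is added to the controller's points, so stronger rebounds score higher.
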(event EventBeginPlay
  (bind _aspc_iron_spin (Utilities|Casting|CastToPC_IronSpin (Game|GetPlayerController 0)))
  (Variables|Default|SetAs%20PC%20Iron%20Spin _aspc_iron_spin))

(event Collision|EventActorBeginOverlap
  (params (OtherActor :type Actor%20Object%20Reference)))

(event EventTick
  (params (DeltaSeconds :type Float%20%28single-precision%29)))

(event Collision|EventHit
  (params (MyComp :type Primitive%20Component%20Object%20Reference) (Other :type Actor%20Object%20Reference) (OtherComp :type Primitive%20Component%20Object%20Reference) (bSelfMoved :type Boolean) (HitLocation :type Vector :default "0, 0, 0") (HitNormal :type Vector :default "0, 0, 0") (NormalImpulse :type Vector :default "0, 0, 0") (Hit :type Hit%20Result%20Structure%20%28by%20ref%29))
  (Physics|AddImpulseatLocation OtherComp (* HitNormal -1e+03 (Variables|Default|GetReboundStrenght)) HitLocation "None")
  (Default|AddPoints (Variables|Default|GetAs%20PC%20Iron%20Spin) (Math|Float|Truncate (Variables|Default|GetReboundStrenght))))

(fn ConstructionScript)