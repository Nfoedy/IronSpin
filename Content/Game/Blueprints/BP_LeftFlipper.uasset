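; BP_LeftFlipper is a physics-driven left flipper, apparently for a pinball-style game, that takes player input from the A button action.
; While the action triggers, it applies a radial velocity-change impulse to the flipper mesh from a scene component's location.
; The physics constraint switches to SLERP angular drive on press and back to Twist and Swing on completion or cancellation.
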(event Input|EnhancedActionEvents|EnhancedInputActionIA_AButton
  (params (ActionValue :type Boolean) (ElapsedSeconds :type Float%20%28double-precision%29) (TriggeredSeconds :type Float%20%28double-precision%29) (InputAction :type Input%20Action%20Object%20Reference :default "/Game/Game/System/Inputs/IA_AButton.IA_AButton"))
  (bind _physicsconstraint (Variables|Default|GetPhysicsConstraint))
  (:Triggered
    (Physics|AddRadialImpulse (Variables|Default|GetStaticMesh) (Transformation|GetWorldLocation (Variables|Default|GetScene)) 5e+02 6e+03 "RIF_Constant" true))
  (:Started
    (Development|PrintString "A")
    (Class|PhysicsConstraintComponent|SetAngularDriveMode _physicsconstraint "SLERP"))
  (:Canceled
    (Class|PhysicsConstraintComponent|SetAngularDriveMode _physicsconstraint "TwistAndSwing" :!label _label))
  (:Completed
    (goto _label)))

(event EventBeginPlay
  (Input|EnableInput (Game|GetPlayerController 0)))

(fn ConstructionScript)