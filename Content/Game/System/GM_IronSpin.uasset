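; GM_IronSpin is the game mode that tracks lives and manages the ball in IronSpin.
; On BeginPlay it fills Lives from MaxLives, takes the first actor of SpawnerClass as the spawner and stores the ball it spawns.
; LoseLife decrements Lives, then either destroys the current ball and spawns a replacement, or calls GameOver.
; GameOver prints a message and pauses the game.
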(event Custom|LoseLife
  (bind _output_get (Variables|Default|SetLives (- (Variables|Default|GetLives) 1)))
  (if (> _output_get 0)
    (CallFunction|RespawnBall)
    (else
      (CallFunction|GameOver))))

(event Custom|RespawnBall
  (if (Utilities|IsValid (Variables|Default|GetBallRef))
    (Actor|DestroyActor (Variables|Default|GetBallRef)))
  (bind _ball (Default|SpawnBall (Variables|Default|GetSpawner)))
  (Variables|Default|SetBallRef _ball))

(event Custom|GameOver
  (Development|PrintString "GAME OVER")
  (Game|SetGamePaused true))

(event EventBeginPlay
  (Variables|Default|SetLives (Variables|Default|GetMaxLives))
  (bind _outactors (Actor|GetAllActorsOfClass (Variables|Default|GetSpawnerClass)))
  (bind _output_get (Variables|Default|SetSpawner (Utilities|Array|Get(acopy) _outactors)))
  (bind _ball (Default|SpawnBall _output_get))
  (Variables|Default|SetBallRef _ball))

(fn ConstructionScript)